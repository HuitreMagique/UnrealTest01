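; Tutorial door Blueprint that slides open via a timeline lerp and closes after a delay once the player leaves its trigger.
; Entering the trigger either opens it directly or, if usable, shows a UI widget and enables Use input for toggling.
; Opening first calls Count on a linked Tutorial_Counter, and stops if that cast fails.
; The construction script applies frame scale, optional mesh and material overrides, and removes the light when disabled.
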(event OnComponentBeginOverlap(TriggerVolume)
  (params (OverlappedComponent :type Primitive%20Component%20Object%20Reference) (OtherActor :type Actor%20Object%20Reference) (OtherComp :type Primitive%20Component%20Object%20Reference) (OtherBodyIndex :type Integer) (bFromSweep :type Boolean) (SweepResult :type Hit%20Result%20Structure%20%28by%20ref%29))
  (Variables|Default|SetPlayerInRange true)
  (if (Variables|DoorSetup|GetDoorIsUsable)
    (UserInterface|Viewport|AddtoViewport (Variables|Default|GetDisplay) 0)
    (Input|EnableInput (Game|GetPlayerController 0))
    (else
      (CallFunction|DoorOpen))))

(event OnComponentEndOverlap(TriggerVolume)
  (params (OverlappedComponent :type Primitive%20Component%20Object%20Reference) (OtherActor :type Actor%20Object%20Reference) (OtherComp :type Primitive%20Component%20Object%20Reference) (OtherBodyIndex :type Integer))
  (Variables|Default|SetPlayerInRange false)
  (Widget|RemovefromParent (Variables|Default|GetDisplay))
  (Utilities|FlowControl|Delay (Variables|DoorSetup|GetCloseDelay))
  (if (not (Variables|Default|GetPlayerInRange))
    (CallFunction|DoorClose)))

(event Custom|DoorClose
  ;[1 0.2359 0.5875] Door open/close motion
  (Variables|Default|SetDoorIsOpen false)
  (bind _driver (Timeline|Timeline_DoorDriver Reverse)
    (:Update
      (Transformation|SetRelativeLocation (Variables|Default|GetDoorRoot) (Math|Vector|Lerp(Vector) (Variables|DoorSetup|GetDoorStart) (Variables|DoorSetup|GetDoorEnd) _driver) false false))))

(event Custom|DoorOpen
  ;[1 0.2359 0.5875] Door open/close motion
  (bind _astutorial_counter (Utilities|Casting|CastToTutorial_Counter (Variables|DoorSetup|GetDoorCounter)))
  (Default|Count _astutorial_counter)
  (Variables|Default|SetDoorIsOpen true)
  (bind _driver (Timeline|Timeline_DoorDriver Play)
    (:Update
      (Transformation|SetRelativeLocation (Variables|Default|GetDoorRoot) (Math|Vector|Lerp(Vector) (Variables|DoorSetup|GetDoorStart) (Variables|DoorSetup|GetDoorEnd) _driver) false false))))

(event EventBeginPlay
  (bind _returnvalue (UserInterface|CreateWidget "/Game/BluePrints/UIDisplay.UIDisplay_C"))
  (Variables|Default|SetDisplay _returnvalue))

(event Collision|EventActorBeginOverlap
  (params (OtherActor :type Actor%20Object%20Reference)))

(event EventTick
  (params (DeltaSeconds :type Float%20%28single-precision%29)))

(event Input|ActionEvents|InputActionUse
  (params (Key :type Key%20Structure :default "AnyKey"))
  (:Pressed
    (if (Variables|Default|GetDoorIsOpen)
      (CallFunction|DoorClose)
      (else
        (CallFunction|DoorOpen)))))

(fn ConstructionScript
  (Transformation|SetRelativeScale3D (Variables|Default|GetFrameRoot) (Math|Conversions|ToVector(Float) (Variables|DoorSetup|Get3D%20Scale)))
  (|StaticMeshOverride)
  (|MaterialOverride)
  (if (not (Variables|DoorSetup|GetLight))
    (Components|DestroyComponent (Variables|Default|GetPointLight))))
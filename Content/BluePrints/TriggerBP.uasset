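; Jump pad trigger actor that launches the player character and animates the pad's material when stepped on.
; The construction script creates a dynamic material instance on the pad mesh.
; On trigger box overlap, it prints the other actor's name, then calls JumpPad on a ThirdPersonPerso and restarts a timeline that drives the scaled "Jump" material parameter.
; Unconnected leftover nodes target ThirdPersonCharacter and set the parameter directly on the mesh.
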(event OnComponentBeginOverlap(TrigBox)
  (params (OverlappedComponent :type Primitive%20Component%20Object%20Reference) (OtherActor :type Actor%20Object%20Reference) (OtherComp :type Primitive%20Component%20Object%20Reference) (OtherBodyIndex :type Integer) (bFromSweep :type Boolean) (SweepResult :type Hit%20Result%20Structure%20%28by%20ref%29))
  (Development|PrintString (Utilities|GetObjectName OtherActor))
  (bind _asthird_person_perso (Utilities|Casting|CastToThirdPersonPerso OtherActor))
  (Default|JumpPad _asthird_person_perso)
  (bind _driver (Timeline|Timeline_0 PlayFromStart)
    (:Update
      (Rendering|Material|SetScalarParameterValue (Variables|Default|GetjumpPadMaterial) "Jump" (* _driver 1e+01) :!class /Script/Engine.MaterialInstanceDynamic))))

(event EventBeginPlay)

(event Collision|EventActorBeginOverlap
  (params (OtherActor :type Actor%20Object%20Reference)))

(event EventTick
  (params (DeltaSeconds :type Float%20%28single-precision%29)))

(fn ConstructionScript
  (bind _jumppadmesh (Variables|Default|GetjumpPadMesh))
  (bind _returnvalue (Rendering|Material|CreateDynamicMaterialInstance _jumppadmesh 0 (Rendering|Material|GetMaterial _jumppadmesh 0) :!class /Script/Engine.PrimitiveComponent))
  (Variables|Default|SetjumpPadMaterial _returnvalue))
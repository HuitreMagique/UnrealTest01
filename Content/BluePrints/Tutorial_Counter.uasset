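; Tutorial counter actor that keeps a running tally of door transactions in DoorTransactions.
; The IncrementDoorTransactions event and the Count function hold identical logic, each adding one to the tally and printing the new value.
; Nothing in this Blueprint calls either one, and its overlap, tick and construction stubs do no work.
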(event Collision|EventActorBeginOverlap
  (params (OtherActor :type Actor%20Object%20Reference)))

(event EventTick
  (params (DeltaSeconds :type Float%20%28single-precision%29)))

(event EventIncrementDoorTransactions
  (bind _output_get (Variables|Default|SetDoorTransactions (+ (Variables|Default|GetDoorTransactions) 1)))
  (Development|PrintString (Utilities|String|ToString(Integer) _output_get)))

(fn ConstructionScript)

(fn Count
  (bind _output_get (Variables|Default|SetDoorTransactions (+ (Variables|Default|GetDoorTransactions) 1)))
  (Development|PrintString (Utilities|String|ToString(Integer) _output_get)))